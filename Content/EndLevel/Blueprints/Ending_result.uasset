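; Ending_result is an end-level results display actor showing a quarterly interim settlement between the user and gurus through text render components.
; SetWindowText compares both percentages for color-coded WIN/LOSE/DRAW, and reads turn and user balance from MyGameInstance.
; The user's percentage gets an arrow, though its zero branch is unreachable behind the >= check.
; The construction script initializes it with zero percentages; event graph events are empty.
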(fn `Set Window Text`
  (params (`Guru's Percent` :type "Float (double-precision)") (`User's Percent` :type "Float (double-precision)"))
  (bind _color (make `Color` 255 0 0 1))
  (bind _color_2 (make `Color` 0 0 255 1))
  (bind _color_3 (make `Color` 0 128))
  (bind _guru_result_text (`self.Guru result Text`))
  (bind _user_result_text (`self.User result Text`))
  (bind _guru_result_text_2 (`self.Guru result Text`))
  (bind _guru_result_text_3 (`self.Guru result Text`))
  (bind _user_amount_percent_text (`self.User amount percent Text`))
  (bind _user_result_text_2 (`self.User result Text`))
  (bind _user_result_text_3 (`self.User result Text`))
  (bind _returnvalue (`KismetTextLibrary.Conv_TextToString` (`KismetTextLibrary.Conv_DoubleToText` `User's Percent` "HalfToEven")))
  (bind _asmy_game_instance (cast `/Game/MainLevel/Blueprints/MyGameInstance` (`GameplayStatics.GetGameInstance`)))
  (`|ExecutionSequence`
    (:`then_0`
      ;[1 1 1] Set Turn Info
      (`TextRenderComponent.K2_SetText` (`self.Turn Text`) (`KismetTextLibrary.Conv_StringToText` (`KismetStringLibrary.Concat_StrStr` (`KismetStringLibrary.Conv_IntToString` (`/Game/MainLevel/Blueprints/MyGameInstance.currentTurn` _asmy_game_instance)) "분기   중간결산"))))
    (:`then_1`
      ;[1 1 1] Set win or lose Info
      (if (> `Guru's Percent` `User's Percent`)
        (`TextRenderComponent.K2_SetText` _user_result_text (`KismetTextLibrary.Conv_StringToText` "LOSE"))
        (`TextRenderComponent.SetTextRenderColor` _user_result_text _color)
        (`TextRenderComponent.K2_SetText` _guru_result_text (`KismetTextLibrary.Conv_StringToText` "WIN"))
        (`TextRenderComponent.SetTextRenderColor` _guru_result_text _color_2)
        (elif (== `Guru's Percent` `User's Percent`)
          (`TextRenderComponent.K2_SetText` _user_result_text_2 (`KismetTextLibrary.Conv_StringToText` "DRAW"))
          (`TextRenderComponent.SetTextRenderColor` _user_result_text_2 _color_3)
          (`TextRenderComponent.K2_SetText` _guru_result_text_3 (`KismetTextLibrary.Conv_StringToText` "DRAW"))
          (`TextRenderComponent.SetTextRenderColor` _guru_result_text_3 _color_3)
          (else
            (`TextRenderComponent.K2_SetText` _user_result_text_3 (`KismetTextLibrary.Conv_StringToText` "WIN"))
            (`TextRenderComponent.SetTextRenderColor` _user_result_text_3 _color_2)
            (`TextRenderComponent.K2_SetText` _guru_result_text_2 (`KismetTextLibrary.Conv_StringToText` "LOSE"))
            (`TextRenderComponent.SetTextRenderColor` _guru_result_text_2 _color)))))
    (:`then_2`
      ;[1 1 1] Set user balance Information
      (if (>= `User's Percent` 0.0)
        (`TextRenderComponent.SetTextRenderColor` _user_amount_percent_text _color_2)
        (`TextRenderComponent.K2_SetText` _user_amount_percent_text (`KismetTextLibrary.Conv_StringToText` (`KismetStringLibrary.Concat_StrStr` "▲" _returnvalue "%")))
        (elif (== `User's Percent` 0.0)
          (`TextRenderComponent.SetTextRenderColor` _user_amount_percent_text (make `Color` 0 128 0 1))
          (`TextRenderComponent.K2_SetText` _user_amount_percent_text (`KismetTextLibrary.Conv_StringToText` (`KismetStringLibrary.Concat_StrStr` "=" _returnvalue "%")))
          (else
            (`TextRenderComponent.SetTextRenderColor` _user_amount_percent_text _color)
            (`TextRenderComponent.K2_SetText` _user_amount_percent_text (`KismetTextLibrary.Conv_StringToText` (`KismetStringLibrary.Concat_StrStr` "▼" _returnvalue "%")))))))
    (:`then_3`
      (`TextRenderComponent.K2_SetText` (`self.User amount Text`) (`KismetTextLibrary.Conv_StringToText` (`KismetStringLibrary.Concat_StrStr` (`KismetTextLibrary.Conv_TextToString` (`KismetTextLibrary.Conv_DoubleToText` (`/Game/MainLevel/Blueprints/MyGameInstance.User_balance` _asmy_game_instance) "HalfToEven")) "$"))))))

(fn `UserConstructionScript`
  (`self.Set Window Text` 0.0))