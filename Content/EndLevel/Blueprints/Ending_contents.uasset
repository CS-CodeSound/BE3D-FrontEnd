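; Ending-screen result panel that shows the final balance and return of the player or the selected guru.
; SetUserResultText and SetGuruResultText read MyGameInstance to fill the name, balance and percent texts.
; The percent is the balance change from StartBalance times 0.01, colored red, green or blue with a symbol for gain, even or loss.
; TextAppear reveals the text components in stages using chained delays.
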(event `TextAppear`
  ;[1 1 1] 글자 나타나기 연출
  (`SceneComponent.SetVisibility` (`self.Name_Text`) true false)
  (`KismetSystemLibrary.Delay` 1.0)
  (`SceneComponent.SetVisibility` (`self.MiddleLine`) true false)
  (`KismetSystemLibrary.Delay` 1.0)
  (`SceneComponent.SetVisibility` (`self.start_info`) true true)
  (`KismetSystemLibrary.Delay` 0.7)
  (`SceneComponent.SetVisibility` (`self.pointer_info`) true false)
  (`KismetSystemLibrary.Delay` 0.7)
  (`SceneComponent.SetVisibility` (`self.end_info`) true true)
  (`KismetSystemLibrary.Delay` 2.0)
  (`SceneComponent.SetVisibility` (`self.percent_info`) true true))

(fn `SetGuruResultText`
  (bind _end_percent_text (`self.end_percent_text`))
  (bind _asmy_game_instance (cast `/Game/MainLevel/Blueprints/MyGameInstance` (`GameplayStatics.GetGameInstance`)))
  (`|ExecutionSequence`
    (:`then_0`
      ;[1 1 1] Set Name Text
      (`TextRenderComponent.K2_SetText` (`self.Name_Text`) (`KismetTextLibrary.Conv_StringToText` (`|GetArrayItem` (`/Game/MainLevel/Blueprints/MyGameInstance.guruList` _asmy_game_instance) (`/Game/MainLevel/Blueprints/MyGameInstance.select_guru_id` _asmy_game_instance)))))
    (:`then_1`
      (bind _guru_balance (`/Game/MainLevel/Blueprints/MyGameInstance.Guru_balance` _asmy_game_instance))
      ;[1 1 1] Set End Balance
      (`TextRenderComponent.K2_SetText` (`self.end_balance_text`) (`KismetTextLibrary.Conv_StringToText` (`KismetStringLibrary.Concat_StrStr` (`KismetStringLibrary.Conv_DoubleToString` _guru_balance) "$"))))
    (:`then_2`
      (bind _returnvalue (* (- _guru_balance (`self.start_balance`)) 0.01))
      ;[1 1 1] Set Percent Text
      (if (> _returnvalue 0.0)
        (`TextRenderComponent.SetTextRenderColor` _end_percent_text (make `Color` 0 0 255 1))
        (bind _returnvalue_2 (`KismetTextLibrary.Conv_TextToString` (`KismetTextLibrary.Conv_StringToText` (`KismetStringLibrary.Conv_DoubleToString` _returnvalue))))
        (`TextRenderComponent.K2_SetText` _end_percent_text (`KismetTextLibrary.Conv_StringToText` (`KismetStringLibrary.Concat_StrStr` "▲" _returnvalue_2 "%")))
        (elif (== _returnvalue 0.0)
          (`TextRenderComponent.SetTextRenderColor` _end_percent_text (make `Color` 0 128 0 1))
          (`TextRenderComponent.K2_SetText` _end_percent_text (`KismetTextLibrary.Conv_StringToText` (`KismetStringLibrary.Concat_StrStr` "=" _returnvalue_2 "%")))
          (else
            (`TextRenderComponent.SetTextRenderColor` _end_percent_text (make `Color` 255 0 0 1))
            (`TextRenderComponent.K2_SetText` _end_percent_text (`KismetTextLibrary.Conv_StringToText` (`KismetStringLibrary.Concat_StrStr` "▼" _returnvalue_2 "%")))))))))

(fn `SetUserResultText`
  (bind _end_percent_text (`self.end_percent_text`))
  (bind _asmy_game_instance (cast `/Game/MainLevel/Blueprints/MyGameInstance` (`GameplayStatics.GetGameInstance`)))
  (`|ExecutionSequence`
    (:`then_0`
      ;[1 1 1] Set Name Text
      (`TextRenderComponent.K2_SetText` (`self.Name_Text`) (`KismetTextLibrary.Conv_StringToText` "Player")))
    (:`then_1`
      (bind _user_balance (`/Game/MainLevel/Blueprints/MyGameInstance.User_balance` _asmy_game_instance))
      ;[1 1 1] Set End Balance
      (`TextRenderComponent.K2_SetText` (`self.end_balance_text`) (`KismetTextLibrary.Conv_StringToText` (`KismetStringLibrary.Concat_StrStr` (`KismetStringLibrary.Conv_DoubleToString` _user_balance) "$"))))
    (:`then_2`
      (bind _returnvalue (* (- _user_balance (`self.start_balance`)) 0.01))
      ;[1 1 1] Set Percent Text
      (set `self.percent` _returnvalue)
      (if (> _returnvalue 0.0)
        (`TextRenderComponent.SetTextRenderColor` _end_percent_text (make `Color` 0 0 255 1))
        (bind _returnvalue_2 (`KismetTextLibrary.Conv_TextToString` (`KismetTextLibrary.Conv_StringToText` (`KismetStringLibrary.Conv_DoubleToString` _returnvalue))))
        (`TextRenderComponent.K2_SetText` _end_percent_text (`KismetTextLibrary.Conv_StringToText` (`KismetStringLibrary.Concat_StrStr` "▲" _returnvalue_2 "%")))
        (elif (== _returnvalue 0.0)
          (`TextRenderComponent.SetTextRenderColor` _end_percent_text (make `Color` 0 128 0 1))
          (`TextRenderComponent.K2_SetText` _end_percent_text (`KismetTextLibrary.Conv_StringToText` (`KismetStringLibrary.Concat_StrStr` "=" _returnvalue_2 "%")))
          (else
            (`TextRenderComponent.SetTextRenderColor` _end_percent_text (make `Color` 255 0 0 1))
            (`TextRenderComponent.K2_SetText` _end_percent_text (`KismetTextLibrary.Conv_StringToText` (`KismetStringLibrary.Concat_StrStr` "▼" _returnvalue_2 "%")))))))))

(fn `UserConstructionScript`)