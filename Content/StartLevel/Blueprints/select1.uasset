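; A start-level selection button actor that lets a VR pawn choose a guru.
; Box overlap flags the VRPawn as hovering over a button and passes it this actor's GuruId; end overlap also sets the hover flag true, never clearing it.
; OpenMainLevel stores a hardcoded guru ID in MyGameInstance and opens MainMap, but nothing here calls it, and the Cube click event is empty.
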(event `self.ReceiveBeginPlay`)

(event `self.Cube.OnClicked`
  (params (TouchedComponent :type "PrimitiveComponent Object Reference") (ButtonPressed :type "Key Structure")))

(event `self.Box.OnComponentBeginOverlap`
  (params (OverlappedComponent :type "PrimitiveComponent Object Reference") (OtherActor :type "Actor Object Reference") (OtherComp :type "PrimitiveComponent Object Reference") (OtherBodyIndex :type Integer) (bFromSweep :type Boolean) (SweepResult :type "HitResult Structure (by ref)"))
  (bind _asvrpawn (cast `/Game/VRTemplate/Blueprints/VRPawn` OtherActor))
  (set `/Game/VRTemplate/Blueprints/VRPawn.IsHoveringOverButton` true _asvrpawn)
  (set `/Game/VRTemplate/Blueprints/VRPawn.selectedGuruId` (`self.guruId`) _asvrpawn))

(event `self.Box.OnComponentEndOverlap`
  (params (OverlappedComponent :type "PrimitiveComponent Object Reference") (OtherActor :type "Actor Object Reference") (OtherComp :type "PrimitiveComponent Object Reference") (OtherBodyIndex :type Integer))
  (bind _asvrpawn (cast `/Game/VRTemplate/Blueprints/VRPawn` OtherActor))
  (set `/Game/VRTemplate/Blueprints/VRPawn.IsHoveringOverButton` true _asvrpawn))

(fn `OpenMainLevel`
  (bind _asmy_game_instance (cast `/Game/MainLevel/Blueprints/MyGameInstance` (`GameplayStatics.GetGameInstance`)))
  (set `/Game/MainLevel/Blueprints/MyGameInstance.select_guru_id` 1 _asmy_game_instance)
  (`GameplayStatics.OpenLevel` "MainMap"))

(fn `UserConstructionScript`)