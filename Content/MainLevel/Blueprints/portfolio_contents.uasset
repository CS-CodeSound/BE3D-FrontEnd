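; Actor that displays one investment portfolio in the level through text render components: name, ten tickers, balance and percent change.
; SetPortfolioValues is its only logic, writing the passed values into those texts, with ticker slots filled by fixed index and a dollar sign after the balance.
; The percent gets an arrow or equals sign and is colored red for gains, green for no change and blue for losses.
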(event `self.ReceiveBeginPlay`)

(fn `Set Portfolio Values`
  (params (Name :type String) (`Ticker List` :type "Array of String") (balance :type "Float (double-precision)") (percent :type "Float (double-precision)"))
  (bind _percent_text (`self.Percent_Text`))
  (bind _returnvalue (`KismetTextLibrary.Conv_TextToString` (`KismetTextLibrary.Conv_DoubleToText` percent "HalfToEven")))
  ;[1 1 1] Set Name
  (`TextRenderComponent.K2_SetText` (`self.Name_Text`) (`KismetTextLibrary.Conv_StringToText` Name))
  ;[1 1 1] Set Tickers
  (`|ExecutionSequence`
    (:`then_0`
      (`TextRenderComponent.K2_SetText` (`self.ticker1`) (`KismetTextLibrary.Conv_StringToText` (`|GetArrayItem` `Ticker List`))))
    (:`then_1`
      (`TextRenderComponent.K2_SetText` (`self.ticker2`) (`KismetTextLibrary.Conv_StringToText` (`|GetArrayItem` `Ticker List` 1))))
    (:`then_2`
      (`TextRenderComponent.K2_SetText` (`self.ticker3`) (`KismetTextLibrary.Conv_StringToText` (`|GetArrayItem` `Ticker List` 2))))
    (:`then_3`
      (`TextRenderComponent.K2_SetText` (`self.ticker4`) (`KismetTextLibrary.Conv_StringToText` (`|GetArrayItem` `Ticker List` 3))))
    (:`then_4`
      (`TextRenderComponent.K2_SetText` (`self.ticker5`) (`KismetTextLibrary.Conv_StringToText` (`|GetArrayItem` `Ticker List` 4))))
    (:`then_5`
      (`TextRenderComponent.K2_SetText` (`self.ticker6`) (`KismetTextLibrary.Conv_StringToText` (`|GetArrayItem` `Ticker List` 5))))
    (:`then_6`
      (`TextRenderComponent.K2_SetText` (`self.ticker7`) (`KismetTextLibrary.Conv_StringToText` (`|GetArrayItem` `Ticker List` 6))))
    (:`then_7`
      (`TextRenderComponent.K2_SetText` (`self.ticker8`) (`KismetTextLibrary.Conv_StringToText` (`|GetArrayItem` `Ticker List` 7))))
    (:`then_8`
      (`TextRenderComponent.K2_SetText` (`self.ticker9`) (`KismetTextLibrary.Conv_StringToText` (`|GetArrayItem` `Ticker List` 8))))
    (:`then_9`
      (`TextRenderComponent.K2_SetText` (`self.ticker10`) (`KismetTextLibrary.Conv_StringToText` (`|GetArrayItem` `Ticker List` 9))))
    (:`then_10`
      ;[1 1 1] Set Balance
      (`TextRenderComponent.K2_SetText` (`self.Balance_Text`) (`KismetTextLibrary.Conv_StringToText` (`KismetStringLibrary.Concat_StrStr` (`KismetTextLibrary.Conv_TextToString` (`KismetTextLibrary.Conv_DoubleToText` balance "HalfToEven")) "$")))
      ;[1 1 1] Set Percent
      (if (> percent 0.0)
        (`TextRenderComponent.SetTextRenderColor` _percent_text (make `Color` 0 0 255 1))
        (`TextRenderComponent.K2_SetText` _percent_text (`KismetTextLibrary.Conv_StringToText` (`KismetStringLibrary.Concat_StrStr` "▲" _returnvalue "%")))
        (elif (== percent 0.0)
          (`TextRenderComponent.SetTextRenderColor` _percent_text (make `Color` 0 128 0 1))
          (`TextRenderComponent.K2_SetText` _percent_text (`KismetTextLibrary.Conv_StringToText` (`KismetStringLibrary.Concat_StrStr` "=" _returnvalue "%")))
          (else
            (`TextRenderComponent.SetTextRenderColor` _percent_text (make `Color` 255 0 0 1))
            (`TextRenderComponent.K2_SetText` _percent_text (`KismetTextLibrary.Conv_StringToText` (`KismetStringLibrary.Concat_StrStr` "▼" _returnvalue "%")))))))))

(fn `UserConstructionScript`)