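; Card Blueprint that spawns stock ticker and analyst display actors from JSON financial data when play begins.
; BeginPlay reads the JSON into a struct and loops over its category keys, spawning a CardText and an InvestmentAnalyst for each.
; CardText receives the ticker, and InvestmentAnalyst receives the rating at index 1 of that ticker's data.
; UpdateCardContent, Tick and overlap handling are empty, and the 13F and category-array lookups are unused.
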(event `self.ReceiveBeginPlay`
  (bind _ticker (`self.ticker`))
  (bind (_boutsuccess _outinfomessage _returnvalue) (`ReadWriteJson.ReadStructFromJsonFile` (`self.String`)))
  (bind (_categories _tickers _pt13fdata) (break `BE3DTestStruct` _returnvalue))
  (bind _keys (`BlueprintMapLibrary.Map_Keys` _categories))
  (for _ _keys
    (bind _returnvalue_2 (`|SpawnActorFromClass` "/Game/MainLevel/Blueprints/CardText.CardText_C" (`self.transform`) "Undefined" "MultiplyWithRoot" null null))
    (`/Game/MainLevel/Blueprints/CardText.SetCardText` _returnvalue_2 _ticker)
    (bind _returnvalue_3 (`|SpawnActorFromClass` "/Game/MainLevel/Blueprints/InvestmentAnalyst.InvestmentAnalyst_C" (`self.transform`) "Undefined" "MultiplyWithRoot" null null))
    (`/Game/MainLevel/Blueprints/InvestmentAnalyst.SetAnalystText` _returnvalue_3 (`|GetArrayItem` (`.Ratings` (break `TickerData` (`BlueprintMapLibrary.Map_Find` _tickers _ticker))) 1))))

(fn `UpdateCardContent`)

(fn `UserConstructionScript`)