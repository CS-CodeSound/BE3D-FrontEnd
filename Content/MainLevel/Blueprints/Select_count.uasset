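; Actor that displays how many cards are selected for purchase, using front and back text render components.
; SetText reads the length of CardsToBuy from MyGameInstance, writes it to the front text, and turns both texts red at ten or more, otherwise black.
; A failed cast only applies the black color.
; The event graph is empty, so nothing in this Blueprint triggers the refresh itself.
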(fn `SetText`
  (bind _color (make `Color` 0 0 0 1))
  (bind _color_2 (make `Color` 0 0 255 1))
  (bind _count_text (`self.Count_text`))
  (bind _count_text_back (`self.Count_text_back`))
  (bind _asmy_game_instance (cast `/Game/MainLevel/Blueprints/MyGameInstance` (`GameplayStatics.GetGameInstance`))
    (:`then`
      (bind _returnvalue (`KismetArrayLibrary.Array_Length` (`/Game/MainLevel/Blueprints/MyGameInstance.CardsToBuy` _asmy_game_instance)))
      (`TextRenderComponent.K2_SetText` _count_text (`KismetTextLibrary.Conv_IntToText` _returnvalue))
      (if (>= _returnvalue 10)
        (`TextRenderComponent.SetTextRenderColor` _count_text _color_2)
        (`TextRenderComponent.SetTextRenderColor` _count_text_back _color_2)
        (else
          (`TextRenderComponent.SetTextRenderColor` _count_text _color :!label _label)
          (`TextRenderComponent.SetTextRenderColor` _count_text_back _color))))
    (:`CastFailed`
      (goto _label))))

(fn `UserConstructionScript`)