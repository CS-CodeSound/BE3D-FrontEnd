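; Actor that labels the Y axes of the earnings graphs for revenue and EPS.
; Two functions each set a bottom and top text label from the GraphYaxisDiff array on MyGameInstance.
; Revenue pins its bottom at zero and reads only the upper value, while EPS reads both bounds.
; The event graph and construction script are empty, so labels update only when these functions are called.
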(event `self.ReceiveBeginPlay`)

(fn `SetEPSYaxis`
  (bind _asmy_game_instance (cast `/Game/MainLevel/Blueprints/MyGameInstance` (`GameplayStatics.GetGameInstance`)))
  (bind _graphyaxisdiff (`/Game/MainLevel/Blueprints/MyGameInstance.graphYaxisDiff` _asmy_game_instance))
  (`TextRenderComponent.K2_SetText` (`self.EPSYaxisBottom`) (`KismetTextLibrary.Conv_DoubleToText` (`|GetArrayItem` _graphyaxisdiff) "HalfToEven"))
  (`TextRenderComponent.K2_SetText` (`self.EPSYaxisTop`) (`KismetTextLibrary.Conv_DoubleToText` (`|GetArrayItem` _graphyaxisdiff 1) "HalfToEven")))

(fn `SetRevenueYaxis`
  (bind _asmy_game_instance (cast `/Game/MainLevel/Blueprints/MyGameInstance` (`GameplayStatics.GetGameInstance`)))
  (`TextRenderComponent.K2_SetText` (`self.RevenueYaxisBottom`) (`KismetTextLibrary.Conv_DoubleToText` 0.0 "HalfToEven"))
  (`TextRenderComponent.K2_SetText` (`self.RevenueYaxisTop`) (`KismetTextLibrary.Conv_DoubleToText` (`|GetArrayItem` (`/Game/MainLevel/Blueprints/MyGameInstance.graphYaxisDiff` _asmy_game_instance) 1) "HalfToEven")))

(fn `UserConstructionScript`)