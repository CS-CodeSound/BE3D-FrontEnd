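; BP_Button is a VR push button that resets movable actors to stored locations.
; When a VRPawn overlaps its box, the button sinks slightly, then rises back when the overlap ends.
; A press pairs actors tagged MovableActor with the GameInstance's InitialLocations by iteration order, teleporting each and setting a fixed rotation.
; Disconnected nodes for opening and closing a settlement modal widget never run.
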(event `self.ReceiveBeginPlay`
  (set `self.ButtonStart` (`SceneComponent.RelativeLocation` (`self.Button`))))

(event `self.Box.OnComponentBeginOverlap`
  (params (OverlappedComponent :type "PrimitiveComponent Object Reference") (OtherActor :type "Actor Object Reference") (OtherComp :type "PrimitiveComponent Object Reference") (OtherBodyIndex :type Integer) (bFromSweep :type Boolean) (SweepResult :type "HitResult Structure (by ref)"))
  (cast `/Game/VRTemplate/Blueprints/VRPawn` OtherActor)
  (`KismetSystemLibrary.MoveComponentTo` (`self.Button`) (- (`self.ButtonStart`) (0.0 0.0 5.0)) (struct) false false 0.1)
  (`KismetSystemLibrary.PrintString` "push")
  (bind _asmy_game_instance (cast `/Game/MainLevel/Blueprints/MyGameInstance` (`GameplayStatics.GetGameInstance`)))
  (for (_array_element _array_index) (`/Game/MainLevel/Blueprints/MyGameInstance.InitialLocations` _asmy_game_instance)
    (bind _outactors (`GameplayStatics.GetAllActorsOfClass` "/Script/Engine.Actor"))
    (set `self.LocationIndex` -1)
    (for _array_element_2 _outactors
      (if (`self.ActorHasTag` _array_element_2 "MovableActor")
        (bind _output_get (set `self.LocationIndex` (+ (`self.LocationIndex`) 1)))
        (if (== _output_get _array_index)
          (`self.K2_SetActorLocation` _array_element_2 _array_element false false)
          (`self.K2_SetActorRotation` _array_element_2 (struct :`Yaw` 90.0) false))))))

(event `self.Box.OnComponentEndOverlap`
  (params (OverlappedComponent :type "PrimitiveComponent Object Reference") (OtherActor :type "Actor Object Reference") (OtherComp :type "PrimitiveComponent Object Reference") (OtherBodyIndex :type Integer))
  (cast `/Game/VRTemplate/Blueprints/VRPawn` OtherActor)
  (`KismetSystemLibrary.MoveComponentTo` (`self.Button`) (`self.ButtonStart`) (struct) false false 0.1))

(fn `UserConstructionScript`)