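; BP_TurnEndButton is a VR turn-end button that also provides the function for showing turn results for a guru and the user.
; The button mesh sinks while a VRPawn overlaps its box and rises on exit.
; CreateTurnendWindow applies both profit percentages to the GameInstance balances, then spawns a summary window with two attached portfolio panels.
; Nothing in this Blueprint calls that function; the press only animates.
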(event `self.ReceiveBeginPlay`
  (set `self.Button Start` (`SceneComponent.RelativeLocation` (`self.Button`))))

(event `self.Box.OnComponentBeginOverlap`
  (params (OverlappedComponent :type "PrimitiveComponent Object Reference") (OtherActor :type "Actor Object Reference") (OtherComp :type "PrimitiveComponent Object Reference") (OtherBodyIndex :type Integer) (bFromSweep :type Boolean) (SweepResult :type "HitResult Structure (by ref)"))
  (cast `/Game/VRTemplate/Blueprints/VRPawn` OtherActor)
  (`KismetSystemLibrary.MoveComponentTo` (`self.Button`) (- (`self.Button Start`) (0.0 0.0 5.0)) (struct) false false 0.1))

(event `self.Box.OnComponentEndOverlap`
  (params (OverlappedComponent :type "PrimitiveComponent Object Reference") (OtherActor :type "Actor Object Reference") (OtherComp :type "PrimitiveComponent Object Reference") (OtherBodyIndex :type Integer))
  (cast `/Game/VRTemplate/Blueprints/VRPawn` OtherActor)
  (`KismetSystemLibrary.MoveComponentTo` (`self.Button`) (`self.Button Start`) (struct) false false 0.1))

(fn `Create_turnend_window`
  (params (`Guru's Pick` :type "Array of String") (`Guru's Profit percent` :type "Float (double-precision)") (`User's Profit percent` :type "Float (double-precision)"))
  (bind _asmy_game_instance (cast `/Game/MainLevel/Blueprints/MyGameInstance` (`GameplayStatics.GetGameInstance`)))
  (bind _returnvalue (`|SpawnActorFromClass` "/Game/MainLevel/Blueprints/Portfolio_Window.Portfolio_Window_C" (`self.Turnend_window_transform`) "Undefined" "MultiplyWithRoot" null null))
  (`|ExecutionSequence`
    (:`then_0`
      (bind _guru_balance (`/Game/MainLevel/Blueprints/MyGameInstance.Guru_balance` _asmy_game_instance))
      ;[1 1 1] set guru's portfolio
      ;;[1 1 1] Guru's 잔고 계산
      (bind _output_get (set `/Game/MainLevel/Blueprints/MyGameInstance.Guru_balance` (+ (* _guru_balance (/ `Guru's Profit percent` 100.0)) _guru_balance) _asmy_game_instance)))
    (:`then_1`
      (bind _user_balance (`/Game/MainLevel/Blueprints/MyGameInstance.User_balance` _asmy_game_instance))
      ;[1 1 1] set user's portfolio
      ;;[1 1 1] User's 잔고 계산
      (bind _output_get_2 (set `/Game/MainLevel/Blueprints/MyGameInstance.User_balance` (+ (* _user_balance (/ `User's Profit percent` 100.0)) _user_balance) _asmy_game_instance)))
    (:`then_2`
      (`/Game/MainLevel/Blueprints/Portfolio_Window.Set Window Text` _returnvalue `Guru's Profit percent` `User's Profit percent`))
    (:`then_3`
      (bind _returnvalue_2 (`|SpawnActorFromClass` "/Game/MainLevel/Blueprints/portfolio_contents.portfolio_contents_C" (`self.guru_portfolio_transform`) "Undefined" "MultiplyWithRoot" null null))
      (`/Game/MainLevel/Blueprints/portfolio_contents.Set Portfolio Values` _returnvalue_2 (`|GetArrayItem` (`/Game/MainLevel/Blueprints/MyGameInstance.guruList` _asmy_game_instance) (`/Game/MainLevel/Blueprints/MyGameInstance.guruIndex` _asmy_game_instance)) `Guru's Pick` _output_get `Guru's Profit percent`)
      (`self.K2_AttachToActor` _returnvalue_2 _returnvalue "None" "KeepRelative" "KeepRelative" "KeepRelative" true))
    (:`then_4`
      (bind _returnvalue_3 (`|SpawnActorFromClass` "/Game/MainLevel/Blueprints/portfolio_contents.portfolio_contents_C" (`self.user_portfolio_transform`) "Undefined" "MultiplyWithRoot" null null))
      (`/Game/MainLevel/Blueprints/portfolio_contents.Set Portfolio Values` _returnvalue_3 "User" (`/Game/MainLevel/Blueprints/MyGameInstance.CardsToBuy` _asmy_game_instance) _output_get_2 `User's Profit percent`)
      (`self.K2_AttachToActor` _returnvalue_3 _returnvalue "None" "KeepRelative" "KeepRelative" "KeepRelative" true))))

(fn `UserConstructionScript`)