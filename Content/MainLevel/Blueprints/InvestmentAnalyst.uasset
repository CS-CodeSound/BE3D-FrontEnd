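; InvestmentAnalyst is an actor that displays five analyst ratings: analyst, company action, price-target action, current and prior adjusted targets, and current and prior ratings.
; SetAnalystText receives five rating records and writes their fields to matching text components; the event graph is empty.
; Only the first record's fields get empty checks.
; The other four rows update unchecked, and only when the first record's RatingPrior is non-empty.
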(fn `SetAnalystText`
  (params (rating0 :type "RatingData Structure") (rating1 :type "RatingData Structure") (rating2 :type "RatingData Structure") (rating3 :type "RatingData Structure") (rating4 :type "RatingData Structure"))
  (bind (_year _month _day _analyst _ratingcurrent _ratingprior _adjustedptcurrent _adjustedptprior _actioncompany _actionpt) (break `RatingData` rating0))
  (bind (_year_2 _month_2 _day_2 _analyst_2 _ratingcurrent_2 _ratingprior_2 _adjustedptcurrent_2 _adjustedptprior_2 _actioncompany_2 _actionpt_2) (break `RatingData` rating1))
  (bind (_year_3 _month_3 _day_3 _analyst_3 _ratingcurrent_3 _ratingprior_3 _adjustedptcurrent_3 _adjustedptprior_3 _actioncompany_3 _actionpt_3) (break `RatingData` rating2))
  (bind (_year_4 _month_4 _day_4 _analyst_4 _ratingcurrent_4 _ratingprior_4 _adjustedptcurrent_4 _adjustedptprior_4 _actioncompany_4 _actionpt_4) (break `RatingData` rating3))
  (bind (_year_5 _month_5 _day_5 _analyst_5 _ratingcurrent_5 _ratingprior_5 _adjustedptcurrent_5 _adjustedptprior_5 _actioncompany_5 _actionpt_5) (break `RatingData` rating4))
  (bind _returnvalue (`KismetTextLibrary.Conv_StringToText` _actioncompany))
  (bind _returnvalue_2 (`KismetTextLibrary.Conv_StringToText` _actionpt))
  (bind _returnvalue_3 (`KismetTextLibrary.Conv_StringToText` _adjustedptcurrent))
  (bind _returnvalue_4 (`KismetTextLibrary.Conv_StringToText` _adjustedptprior))
  (bind _returnvalue_5 (`KismetTextLibrary.Conv_StringToText` _analyst))
  (bind _returnvalue_6 (`KismetTextLibrary.Conv_StringToText` _ratingcurrent))
  (bind _returnvalue_7 (`KismetTextLibrary.Conv_StringToText` _ratingprior))
  (if (not (`KismetTextLibrary.TextIsEmpty` _returnvalue))
    (`TextRenderComponent.K2_SetText` (`self.ActionCompany`) _returnvalue))
  (if (not (`KismetTextLibrary.TextIsEmpty` _returnvalue_2))
    (`TextRenderComponent.K2_SetText` (`self.ActionPt`) _returnvalue_2))
  (if (not (`KismetTextLibrary.TextIsEmpty` _returnvalue_3))
    (`TextRenderComponent.K2_SetText` (`self.AdjustedPtCurrent`) _returnvalue_3))
  (if (not (`KismetTextLibrary.TextIsEmpty` _returnvalue_4))
    (`TextRenderComponent.K2_SetText` (`self.AdjustedPtPrior`) _returnvalue_4))
  (if (not (`KismetTextLibrary.TextIsEmpty` _returnvalue_5))
    (`TextRenderComponent.K2_SetText` (`self.AnanlystCompany`) _returnvalue_5))
  (if (not (`KismetTextLibrary.TextIsEmpty` _returnvalue_6))
    (`TextRenderComponent.K2_SetText` (`self.RaitingCurrent`) _returnvalue_6))
  (if (not (`KismetTextLibrary.TextIsEmpty` _returnvalue_7))
    (`TextRenderComponent.K2_SetText` (`self.RatingPrior`) _returnvalue_7)
    (`TextRenderComponent.K2_SetText` (`self.ActionCompany1`) (`KismetTextLibrary.Conv_StringToText` _actioncompany_2))
    (`TextRenderComponent.K2_SetText` (`self.ActionPt1`) (`KismetTextLibrary.Conv_StringToText` _actionpt_2))
    (`TextRenderComponent.K2_SetText` (`self.AdjustedPtCurrent1`) (`KismetTextLibrary.Conv_StringToText` _adjustedptcurrent_2))
    (`TextRenderComponent.K2_SetText` (`self.AdjustedPtPrior1`) (`KismetTextLibrary.Conv_StringToText` _adjustedptprior_2))
    (`TextRenderComponent.K2_SetText` (`self.AnanlystCompany1`) (`KismetTextLibrary.Conv_StringToText` _analyst_2))
    (`TextRenderComponent.K2_SetText` (`self.RaitingCurrent1`) (`KismetTextLibrary.Conv_StringToText` _ratingcurrent_2))
    (`TextRenderComponent.K2_SetText` (`self.RatingPrior1`) (`KismetTextLibrary.Conv_StringToText` _ratingprior_2))
    (`TextRenderComponent.K2_SetText` (`self.ActionCompany2`) (`KismetTextLibrary.Conv_StringToText` _actioncompany_3))
    (`TextRenderComponent.K2_SetText` (`self.ActionPt2`) (`KismetTextLibrary.Conv_StringToText` _actionpt_3))
    (`TextRenderComponent.K2_SetText` (`self.AdjustedPtCurrent2`) (`KismetTextLibrary.Conv_StringToText` _adjustedptcurrent_3))
    (`TextRenderComponent.K2_SetText` (`self.AdjustedPtPrior2`) (`KismetTextLibrary.Conv_StringToText` _adjustedptprior_3))
    (`TextRenderComponent.K2_SetText` (`self.AnanlystCompany2`) (`KismetTextLibrary.Conv_StringToText` _analyst_3))
    (`TextRenderComponent.K2_SetText` (`self.RaitingCurrent2`) (`KismetTextLibrary.Conv_StringToText` _ratingcurrent_3))
    (`TextRenderComponent.K2_SetText` (`self.RatingPrior2`) (`KismetTextLibrary.Conv_StringToText` _ratingprior_3))
    (`TextRenderComponent.K2_SetText` (`self.ActionCompany3`) (`KismetTextLibrary.Conv_StringToText` _actioncompany_4))
    (`TextRenderComponent.K2_SetText` (`self.ActionPt3`) (`KismetTextLibrary.Conv_StringToText` _actionpt_4))
    (`TextRenderComponent.K2_SetText` (`self.AdjustedPtCurrent3`) (`KismetTextLibrary.Conv_StringToText` _adjustedptcurrent_4))
    (`TextRenderComponent.K2_SetText` (`self.AdjustedPtPrior3`) (`KismetTextLibrary.Conv_StringToText` _adjustedptprior_4))
    (`TextRenderComponent.K2_SetText` (`self.AnanlystCompany3`) (`KismetTextLibrary.Conv_StringToText` _analyst_4))
    (`TextRenderComponent.K2_SetText` (`self.RaitingCurrent3`) (`KismetTextLibrary.Conv_StringToText` _ratingcurrent_4))
    (`TextRenderComponent.K2_SetText` (`self.RatingPrior3`) (`KismetTextLibrary.Conv_StringToText` _ratingprior_4))
    (`TextRenderComponent.K2_SetText` (`self.ActionCompany4`) (`KismetTextLibrary.Conv_StringToText` _actioncompany_5))
    (`TextRenderComponent.K2_SetText` (`self.ActionPt4`) (`KismetTextLibrary.Conv_StringToText` _actionpt_5))
    (`TextRenderComponent.K2_SetText` (`self.AdjustedPtCurrent4`) (`KismetTextLibrary.Conv_StringToText` _adjustedptcurrent_5))
    (`TextRenderComponent.K2_SetText` (`self.AdjustedPtPrior4`) (`KismetTextLibrary.Conv_StringToText` _adjustedptprior_5))
    (`TextRenderComponent.K2_SetText` (`self.AnanlystCompany4`) (`KismetTextLibrary.Conv_StringToText` _analyst_5))
    (`TextRenderComponent.K2_SetText` (`self.RaitingCurrent4`) (`KismetTextLibrary.Conv_StringToText` _ratingcurrent_5))
    (`TextRenderComponent.K2_SetText` (`self.RatingPrior4`) (`KismetTextLibrary.Conv_StringToText` _ratingprior_5))))

(fn `UserConstructionScript`)