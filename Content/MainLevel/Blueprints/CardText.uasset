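; CardText is an unfinished Blueprint for showing a card's name on a TextRender component, likely for ticker-based cards.
; BeginPlay calls GetCardName with an empty ticker, but the SetCardText call that would use the result is disconnected, as is the SetText node inside SetCardText.
; GetCardName and GetCardPrice are stubs returning empty strings, and GetCardPrice is never called, so no text is updated at runtime.
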(event `self.ReceiveBeginPlay`
  (bind _cardname (`self.GetCardName` "")))

(fn `GetCardName`
  (params (ticker :type String))
  (returns (CardName :type String))
  (return ""))

(fn `GetCardPrice`
  (params (ticekr :type String))
  (returns (CardPrice :type String))
  (return ""))

(fn `SetCardText`
  (params (CardName :type String)))

(fn `UserConstructionScript`)