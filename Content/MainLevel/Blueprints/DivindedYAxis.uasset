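; Actor that labels the Y axis of a graph with a bottom and a top value.
; SetDividendYaxis reads the first two entries of GraphYaxisDiff from MyGameInstance and writes them as text to YaxisBottom and YaxisTop.
; It does no work on its own events or construction script, so the labels change only when that function is called.
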(event `self.ReceiveBeginPlay`)

(fn `SetDividendYaxis`
  (bind _asmy_game_instance (cast `/Game/MainLevel/Blueprints/MyGameInstance` (`GameplayStatics.GetGameInstance`)))
  (bind _graphyaxisdiff (`/Game/MainLevel/Blueprints/MyGameInstance.graphYaxisDiff` _asmy_game_instance))
  (`TextRenderComponent.K2_SetText` (`self.YaxisBottom`) (`KismetTextLibrary.Conv_DoubleToText` (`|GetArrayItem` _graphyaxisdiff) "HalfToEven"))
  (`TextRenderComponent.K2_SetText` (`self.YaxisTop`) (`KismetTextLibrary.Conv_DoubleToText` (`|GetArrayItem` _graphyaxisdiff 1) "HalfToEven")))

(fn `UserConstructionScript`)