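; BP_Counter displays the counter value stored in the game instance as in-world text through a TextRender component.
; On BeginPlay it calls UpdateCounterValue, which casts the game instance to MyGameInstance, prints CounterValue for debugging and writes it to the text.
; The file only reads the value and refreshes it at BeginPlay, with no Tick or event binding for later changes.
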(event `self.ReceiveBeginPlay`
  (`self.UpdateCounterValue`))

(fn `UpdateCounterValue`
  (bind _asmy_game_instance (cast `/Game/MainLevel/Blueprints/MyGameInstance` (`GameplayStatics.GetGameInstance`)))
  (bind _countervalue (`/Game/MainLevel/Blueprints/MyGameInstance.CounterValue` _asmy_game_instance))
  (`KismetSystemLibrary.PrintString` (`KismetStringLibrary.Conv_IntToString` _countervalue))
  (`TextRenderComponent.K2_SetText` (`self.TextRender`) (`KismetTextLibrary.Conv_StringToText` (`KismetStringLibrary.Conv_IntToString` _countervalue))))

(fn `UserConstructionScript`)