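; BP_SelectButton is a physical VR push button that selects a category by index and shows a configurable text label.
; When the VR pawn overlaps its box, the button mesh slides down slightly, then slides back when the overlap ends.
; On release, it writes its index to the game instance's category and fires the index-changed call if the value differs.
; Disconnected leftover nodes handle a settlement modal widget and debug prints.
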(event `self.ReceiveBeginPlay`
  (set `self.ButtonStart` (`SceneComponent.RelativeLocation` (`self.Button`)))
  (`TextRenderComponent.K2_SetText` (`self.text`) (`KismetTextLibrary.Conv_StringToText` (`self.Button_Text`))))

(event `self.Box.OnComponentBeginOverlap`
  (params (OverlappedComponent :type "PrimitiveComponent Object Reference") (OtherActor :type "Actor Object Reference") (OtherComp :type "PrimitiveComponent Object Reference") (OtherBodyIndex :type Integer) (bFromSweep :type Boolean) (SweepResult :type "HitResult Structure (by ref)"))
  (cast `/Game/VRTemplate/Blueprints/VRPawn` OtherActor)
  (`KismetSystemLibrary.MoveComponentTo` (`self.Button`) (- (`self.ButtonStart`) (0.0 0.0 5.0)) (struct) false false 0.1))

(event `InputAction|CloseWidget`
  (params (Key :type "Key Structure")))

(event `self.Box.OnComponentEndOverlap`
  (params (OverlappedComponent :type "PrimitiveComponent Object Reference") (OtherActor :type "Actor Object Reference") (OtherComp :type "PrimitiveComponent Object Reference") (OtherBodyIndex :type Integer))
  (bind _buttonindex (`self.ButtonIndex`))
  (cast `/Game/VRTemplate/Blueprints/VRPawn` OtherActor)
  (`KismetSystemLibrary.MoveComponentTo` (`self.Button`) (`self.ButtonStart`) (struct) false false 0.1)
  (bind _asmy_game_instance (cast `/Game/MainLevel/Blueprints/MyGameInstance` (`GameplayStatics.GetGameInstance`)))
  (if (!= _buttonindex (`/Game/MainLevel/Blueprints/MyGameInstance.categoryIndex` _asmy_game_instance))
    (set `/Game/MainLevel/Blueprints/MyGameInstance.categoryIndex` _buttonindex _asmy_game_instance)
    (`KismetSystemLibrary.PrintString` "Hello")
    (`/Game/MainLevel/Blueprints/MyGameInstance.OnIndexChanged` _asmy_game_instance)))

(fn `UserConstructionScript`)