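; Card actor Blueprint that shows whether a card is selected for purchase.
; SetCardColor swaps the static mesh material between selected and not-selected variants based on a boolean.
; CheckCardSelected searches the GameInstance's CardsToBuy array for a given ticker, printing the array length to screen and setting IsTickerSelect on a match.
; Event graph, construction script, UpdateText and PublicFunc are empty.
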(event `self.ReceiveBeginPlay`)

(fn `Check Card Selected`
  (params (Ticker :type String))
  (returns (is_ticker_selected :type Boolean))
  (bind _asmy_game_instance (cast `/Game/MainLevel/Blueprints/MyGameInstance` (`GameplayStatics.GetGameInstance`)))
  (bind _cardstobuy (`/Game/MainLevel/Blueprints/MyGameInstance.CardsToBuy` _asmy_game_instance))
  (bind _returnvalue (`KismetArrayLibrary.Array_Length` _cardstobuy))
  (if (!= _returnvalue 0)
    (bind _returnvalue_2 (`KismetStringLibrary.Conv_IntToString` _returnvalue))
    (`KismetSystemLibrary.PrintString` _returnvalue_2 true true (struct :`R` 1.0 :`G` 0.014578 :`A` 1.0) 5.0)
    (for _array_element _cardstobuy
      (if (`KismetStringLibrary.EqualEqual_StrStr` _array_element Ticker)
        (bind _output_get (set `self.is_ticker_select` true))
        (return _output_get)))
    (else
      (`KismetSystemLibrary.PrintString` _returnvalue_2 true true (struct :`R` 1.0 :`G` 0.021375 :`A` 1.0) 5.0)))
  (return false))

(fn `PublicFunc`)

(fn `SetCardColor`
  (params (Color :type Boolean))
  (bind _staticmesh (`self.StaticMesh`))
  (if Color
    (`PrimitiveComponent.SetMaterial` _staticmesh 0 "/Game/MainLevel/Materials/Card_selected.Card_selected")
    (else
      (`PrimitiveComponent.SetMaterial` _staticmesh 0 "/Game/MainLevel/Materials/Card_not_selected.Card_not_selected"))))

(fn `UpdateText`)

(fn `UserConstructionScript`)