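; CardText1 is an actor Blueprint that sets the text of a card's Name component when play begins.
; BeginPlay passes the result of GetCardName to SetCardText, which converts it to text for display.
; GetCardName looks up a hard-coded row in StockTable, ignoring its Ticker input.
; Its return node for the row's Name is unwired, so the looked-up name never reaches the card.
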(event `self.ReceiveBeginPlay`
  (bind _cardname (`self.Get Card Name` ""))
  (`self.SetCardText` _cardname))

(fn `Get Card Name`
  (params (ticker :type String))
  (returns (CardName :type String))
  (bind _returnvalue (`|GetDataTableRow` "/Game/MainLevel/Blueprints/StockTable.StockTable" "1")))

(fn `SetCardText`
  (params (CardName :type String))
  (`TextRenderComponent.K2_SetText` (`self.Name`) (`KismetTextLibrary.Conv_StringToText` CardName))
  (return))

(fn `UserConstructionScript`)